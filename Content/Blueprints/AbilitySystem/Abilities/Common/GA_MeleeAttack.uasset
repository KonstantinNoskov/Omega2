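; GA_MeleeAttack is a common gameplay ability that plays the avatar's melee attack animation.
; On activation it checks the avatar for CombatInterface, gets the attack animation and animation instance through it, and plays the animation as an override.
; It ends immediately without waiting for the animation, and contains no cost commit, hit detection or damage logic.
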(event Ability|EventActivateAbility
  (Utilities|FlowControl|Sequence
    (:then_0
      (Variables|Default|SetCharacter (Ability|GetAvatarActorfromActorInfo)))
    (:then_1
      (if (Utilities|DoesObjectImplementInterface (Variables|Default|GetCharacter) "/Script/Omega.CombatInterface")
        (bind _returnvalue (Class|CombatInterface|GetAttackAnimation(Message) (Variables|Default|GetCharacter)))
        (bind _returnvalue_2 (Class|CombatInterface|GetAnimationInstance(Message) (Variables|Default|GetCharacter)))
        (Class|PaperZDAnimInstance|PlayAnimationOverride _returnvalue_2 _returnvalue "DefaultSlot" 1.0 0.0)))
    (:then_2
      (Ability|EndAbility))))

(event Ability|EventOnEndAbility
  (params (bWasCancelled :type Boolean)))