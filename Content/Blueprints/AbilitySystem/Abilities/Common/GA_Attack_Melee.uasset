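; Common melee attack gameplay ability that damages living players in front of or around the avatar's combat socket.
; On activation, it requires the avatar to implement CombatInterface and sends it the attack message to handle the attack.
; It then applies damage to each player found in a long, narrow box at the socket, ignoring itself, and ends immediately.
; An animation-wait node is present but never runs.
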(event Ability|EventActivateAbility
  (Variables|Default|SetCharacterOwner (Ability|GetAvatarActorfromActorInfo))
  (if (Utilities|DoesObjectImplementInterface (Variables|Default|GetCharacterOwner) "/Script/Omega.CombatInterface")
    (Utilities|FlowControl|Sequence
      (:then_0
        ;[1 0.3944 0.8064] Handle Attack
        (Class|CombatInterface|Attack(Message) (Variables|Default|GetCharacterOwner)))
      (:then_1
        (bind _returnvalue (Class|CombatInterface|GetCombatSocketLocation(Message) (Variables|Default|GetCharacterOwner)))
        (for _array_element (Class|OmegaFunctionLibrary|GetAlivePlayersWithinBox (Variables|Default|GetCharacterOwner) (Utilities|Array|MakeArray (Variables|Default|GetCharacterOwner)) (Math|Vector|MakeVector 2.5e+02 1e+01 5e+01) _returnvalue)
          (Class|OmegaDamageAbility|CauseDamage _array_element)))
      (:then_2
        (Ability|EndAbility)))))