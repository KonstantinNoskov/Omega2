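; GA_Death is a gameplay ability that handles the death of its avatar actor.
; On activation, if the avatar implements CombatInterface, it applies GE_Death to its owner, calls the interface's Die message and ends the ability.
; Disconnected nodes for removing the effect and setting a death Blackboard key never run, so this ability leaves GE_Death applied.
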(event Ability|EventActivateAbility
  (Variables|Default|SetCharacterOwner (Ability|GetAvatarActorfromActorInfo))
  (if (Utilities|DoesObjectImplementInterface (Variables|Default|GetCharacterOwner) "/Script/Omega.CombatInterface")
    (Utilities|FlowControl|Sequence
      (:then_0
        ;[0.4439 1 0.2916] Apply Death Effect
        (bind _returnvalue (Ability|ApplyGameplayEffectToOwner "/Game/Blueprints/AbilitySystem/GameplayEffects/Meta/GE_Death.GE_Death_C"))
        (Variables|Default|SetActive%20GE_Death _returnvalue))
      (:then_1
        ;[1 0.3944 0.8064] Call Combat Interface Die Function
        (Class|CombatInterface|Die(Message) (Variables|Default|GetCharacterOwner)))
      (:then_2)
      (:then_3
        ;[1 0.08209 0.2219] End Ability
        (Ability|EndAbility)))))